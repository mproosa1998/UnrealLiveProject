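; BP_BallGoal is a goal actor that turns the player from a ball back into a human character.
; When an actor tagged Ball hits its GoalForceField, it unpossesses the player controller, spawns an Hour of Code character at SpawnNode and possesses it.
; It then sets IsHuman on the Hour of Code game mode and destroys the ball.
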(event OnComponentHit(GoalForceField)
  (params (HitComponent :type Primitive%20Component%20Object%20Reference) (OtherActor :type Actor%20Object%20Reference) (OtherComp :type Primitive%20Component%20Object%20Reference) (NormalImpulse :type Vector :default "0, 0, 0") (Hit :type Hit%20Result%20Structure%20%28by%20ref%29))
  (bind _spawnnode (Variables|Default|GetSpawnNode))
  (bind _returnvalue (Transformation|GetWorldTransform _spawnnode))
  (if (Actor|ActorHasTag OtherActor "Ball")
    (Pawn|UnPossess (Game|GetPlayerController 0))
    (bind _returnvalue_2 (Game|SpawnActorfromClass "/Game/Hour_of_Code/Blueprints/Game/BP_HourOfCode_Character.BP_HourOfCode_Character_C" (Math|Transform|MakeTransform (.location _returnvalue) (.rotation _returnvalue) "1,1,1") "AlwaysSpawn" 0 0))
    (Pawn|Possess (Game|GetPlayerController 0) _returnvalue_2)
    (bind _asbp_hour_of_code_game (Utilities|Casting|CastToBP_HourOfCode_Game (Game|GetGameMode)))
    (Variables|/Game/Hour_of_Code/Blueprints/Game/BP_HourOfCode_Game.BP_HourOfCode_Game_C|SetisHuman _asbp_hour_of_code_game true)
    (Actor|DestroyActor OtherActor)))

(fn ConstructionScript)