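; Actor that plays a level sequence when five linked buttons are all activated and reverses it when any of them deactivates.
; Tick polls the five ButtonActivated flags on every frame.
; Two DoOnce gates re-arm each other, so each change of the combined state triggers playback only once.
; The forward pass creates the sequence player, and the reverse pass reuses it.
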(event EventTick
  (params (DeltaSeconds :type Float%20%28single-precision%29))
  (if (Math|Boolean|ANDBoolean (Variables|/Game/Hour_of_Code/Blueprints/BP_Button.BP_Button_C|GetButtonActivated (Variables|Default|GetButton1)) (Variables|/Game/Hour_of_Code/Blueprints/BP_Button.BP_Button_C|GetButtonActivated (Variables|Default|GetButton2)) (Variables|/Game/Hour_of_Code/Blueprints/BP_Button.BP_Button_C|GetButtonActivated (Variables|Default|GetButton3)) (Variables|/Game/Hour_of_Code/Blueprints/BP_Button.BP_Button_C|GetButtonActivated (Variables|Default|GetButton4)) (Variables|/Game/Hour_of_Code/Blueprints/BP_Button.BP_Button_C|GetButtonActivated (Variables|Default|GetButton5)))
    (Utilities|FlowControl|DoOnce false :!label _label
      (:Completed
        (bind _outactor (Sequencer|Player|CreateLevelSequencePlayer (Variables|Default|GetSequence)))
        (Sequencer|Player|Play (Variables|/Script/LevelSequence.LevelSequenceActor|GetSequencePlayer _outactor) :!class /Script/MovieScene.MovieSceneSequencePlayer)
        (goto _label_2 Reset)))
    (else
      (Utilities|FlowControl|DoOnce true :!label _label_2
        (:Completed
          (Class|MovieSceneSequencePlayer|PlayReverse (Variables|/Script/LevelSequence.LevelSequenceActor|GetSequencePlayer _outactor))
          (goto _label Reset))))))

(fn ConstructionScript)