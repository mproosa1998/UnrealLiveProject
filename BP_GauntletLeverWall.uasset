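; BP_GauntletLeverWall is a ten-lever combination puzzle that drives a level sequence in the gauntlet.
; Tick checks every lever's LeverActivated against a hard-coded on/off pattern.
; A match creates a sequence player once and starts it looping indefinitely.
; Two DoOnce gates re-arm each other, so breaking the pattern afterwards plays the sequence in reverse once and allows another solve.
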(event EventTick
  (params (DeltaSeconds :type Float%20%28single-precision%29))
  (if (Math|Boolean|ANDBoolean (not (Variables|/Game/Hour_of_Code/Blueprints/BP_Lever.BP_Lever_C|GetLeverActivated (Variables|Default|GetLever_9))) (Variables|/Game/Hour_of_Code/Blueprints/BP_Lever.BP_Lever_C|GetLeverActivated (Variables|Default|GetLever_7)) (Variables|/Game/Hour_of_Code/Blueprints/BP_Lever.BP_Lever_C|GetLeverActivated (Variables|Default|GetLever_4)) (Variables|/Game/Hour_of_Code/Blueprints/BP_Lever.BP_Lever_C|GetLeverActivated (Variables|Default|GetLever_8)) (not (Variables|/Game/Hour_of_Code/Blueprints/BP_Lever.BP_Lever_C|GetLeverActivated (Variables|Default|GetLever_6))) (Variables|/Game/Hour_of_Code/Blueprints/BP_Lever.BP_Lever_C|GetLeverActivated (Variables|Default|GetLever_3)) (not (Variables|/Game/Hour_of_Code/Blueprints/BP_Lever.BP_Lever_C|GetLeverActivated (Variables|Default|GetLever_1))) (Variables|/Game/Hour_of_Code/Blueprints/BP_Lever.BP_Lever_C|GetLeverActivated (Variables|Default|GetLever_10)) (Variables|/Game/Hour_of_Code/Blueprints/BP_Lever.BP_Lever_C|GetLeverActivated (Variables|Default|GetLever_5)) (Variables|/Game/Hour_of_Code/Blueprints/BP_Lever.BP_Lever_C|GetLeverActivated (Variables|Default|GetLever_2)))
    (Utilities|FlowControl|DoOnce false :!label _label
      (:Completed
        (bind _outactor (Sequencer|Player|CreateLevelSequencePlayer (Variables|Default|GetLevelSequence)))
        (Sequencer|Player|Play (Variables|/Script/LevelSequence.LevelSequenceActor|GetSequencePlayer _outactor) :!class /Script/MovieScene.MovieSceneSequencePlayer)
        (Class|MovieSceneSequencePlayer|PlayLooping (Variables|/Script/LevelSequence.LevelSequenceActor|GetSequencePlayer _outactor) -1)
        (goto _label_2 Reset)))
    (else
      (Utilities|FlowControl|DoOnce true :!label _label_2
        (:Completed
          (Class|MovieSceneSequencePlayer|PlayReverse (Variables|/Script/LevelSequence.LevelSequenceActor|GetSequencePlayer _outactor))
          (goto _label Reset))))))

(fn ConstructionScript)