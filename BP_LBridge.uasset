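; Bridge actor driven by two levers, top and bottom, that plays a connected Level Sequence forward or in reverse.
; BeginPlay creates the sequence player once the game mode cast to BP_HourOfCode_Game succeeds.
; Tick polls both levers: either active triggers the other lever's InteractAltStart and plays forward, while both inactive plays in reverse.
; Two DoOnce gates re-arm each other, so each direction fires once per state change.
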(event EventBeginPlay
  (Utilities|Casting|CastToBP_HourOfCode_Game (Game|GetGameMode))
  (bind _outactor (Sequencer|Player|CreateLevelSequencePlayer (Variables|Default|GetConected%20Sequence))))

(event EventTick
  (params (DeltaSeconds :type Float%20%28single-precision%29))
  (if (or (Variables|/Game/Hour_of_Code/Blueprints/BP_Lever.BP_Lever_C|GetLeverActivated (Variables|Default|GetLever_Bottom)) (Variables|/Game/Hour_of_Code/Blueprints/BP_Lever.BP_Lever_C|GetLeverActivated (Variables|Default|GetLever_Top)))
    (Utilities|FlowControl|DoOnce true :!label _label
      (:Completed
        (if (Variables|/Game/Hour_of_Code/Blueprints/BP_Lever.BP_Lever_C|GetLeverActivated (Variables|Default|GetLever_Bottom))
          (Default|InteractAltStart (Variables|Default|GetLever_Top))
          (else
            (Default|InteractAltStart (Variables|Default|GetLever_Bottom))))
        (Sequencer|Player|Play (Variables|/Script/LevelSequence.LevelSequenceActor|GetSequencePlayer (stale EventBeginPlay _outactor)) :!class /Script/MovieScene.MovieSceneSequencePlayer)
        (goto _label_2 Reset)))
    (else
      (Utilities|FlowControl|DoOnce false :!label _label_2
        (:Completed
          (if (Math|Boolean|Equal(Boolean) (Variables|/Game/Hour_of_Code/Blueprints/BP_Lever.BP_Lever_C|GetLeverActivated (Variables|Default|GetLever_Bottom)) (Variables|/Game/Hour_of_Code/Blueprints/BP_Lever.BP_Lever_C|GetLeverActivated (Variables|Default|GetLever_Top)))
            _
            (elif (not (Variables|/Game/Hour_of_Code/Blueprints/BP_Lever.BP_Lever_C|GetLeverActivated (Variables|Default|GetLever_Bottom)))
              (Default|InteractAltStart (Variables|Default|GetLever_Top))
              (else
                (Default|InteractAltStart (Variables|Default|GetLever_Bottom)))))
          (Class|MovieSceneSequencePlayer|PlayReverse (Variables|/Script/LevelSequence.LevelSequenceActor|GetSequencePlayer (stale EventBeginPlay _outactor)))
          (goto _label Reset))))))

(fn ConstructionScript)