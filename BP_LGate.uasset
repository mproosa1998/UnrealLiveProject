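; BP_LGate is a lever-puzzle gate whose force field lowers only while levers 1, 3 and 5 are active and levers 2 and 4 are inactive.
; Tick checks this combination every frame and moves the ForceField component down on a match or back up otherwise.
; Two DoOnce nodes that reset each other make each timed move fire once per change of state.
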(event EventTick
  (params (DeltaSeconds :type Float%20%28single-precision%29))
  (bind _forcefield (Variables|Default|GetForceField))
  (if (Math|Boolean|ANDBoolean (Variables|/Game/Hour_of_Code/Blueprints/BP_Lever.BP_Lever_C|GetLeverActivated (Variables|Default|GetLever_1)) (not (Variables|/Game/Hour_of_Code/Blueprints/BP_Lever.BP_Lever_C|GetLeverActivated (Variables|Default|GetLever_2))) (Variables|/Game/Hour_of_Code/Blueprints/BP_Lever.BP_Lever_C|GetLeverActivated (Variables|Default|GetLever_3)) (not (Variables|/Game/Hour_of_Code/Blueprints/BP_Lever.BP_Lever_C|GetLeverActivated (Variables|Default|GetLever_4))) (Variables|/Game/Hour_of_Code/Blueprints/BP_Lever.BP_Lever_C|GetLeverActivated (Variables|Default|GetLever_5)))
    (Utilities|FlowControl|DoOnce true :!label _label
      (:Completed
        (Components|MoveComponentTo _forcefield "0, 0,-430.000000" "0, 0, 0" false false 1.5 false)
        (goto _label_2 Reset)))
    (else
      (Utilities|FlowControl|DoOnce false :!label _label_2
        (:Completed
          (Components|MoveComponentTo _forcefield "0, 0,-40.000000" "0, 0, 0" false true 2.0 false)
          (goto _label Reset))))))

(fn ConstructionScript)