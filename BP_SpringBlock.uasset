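; BP_SpringBlock is a block that plays a linked level sequence according to the state of a referenced lever.
; BeginPlay creates the sequence player once the game mode casts to BP_HourOfCode_Game.
; Tick polls the lever, playing the sequence forward when activated and in reverse when deactivated.
; Two DoOnce gates reset each other so each change triggers playback only once.
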(event EventBeginPlay
  (Utilities|Casting|CastToBP_HourOfCode_Game (Game|GetGameMode))
  (bind _outactor (Sequencer|Player|CreateLevelSequencePlayer (Variables|Default|GetConected%20Sequence))))

(event EventTick
  (params (DeltaSeconds :type Float%20%28single-precision%29))
  (if (Variables|/Game/Hour_of_Code/Blueprints/BP_Lever.BP_Lever_C|GetLeverActivated (Variables|Default|GetLever))
    (Utilities|FlowControl|DoOnce true :!label _label
      (:Completed
        (Sequencer|Player|Play (Variables|/Script/LevelSequence.LevelSequenceActor|GetSequencePlayer (stale EventBeginPlay _outactor)) :!class /Script/MovieScene.MovieSceneSequencePlayer)
        (goto _label_2 Reset)))
    (else
      (Utilities|FlowControl|DoOnce false :!label _label_2
        (:Completed
          (Class|MovieSceneSequencePlayer|PlayReverse (Variables|/Script/LevelSequence.LevelSequenceActor|GetSequencePlayer (stale EventBeginPlay _outactor)))
          (goto _label Reset))))))

(fn ConstructionScript)