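; Grappling hook equipment that pulls the player toward a hit point, or pulls objects tagged CanBeGrappled toward the player.
; Activate line-traces from the follow camera, attaches the hook to the hit actor, shows the cable and spins the reel.
; Tick drives the pull by setting character velocity or offsetting the object, and feeds the hook location to the character AnimBP.
; Cancel, also triggered when the player overlaps HookCancelTrigger, resets everything.
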(event OnComponentBeginOverlap(HookCancelTrigger)
  (params (OverlappedComponent :type Primitive%20Component%20Object%20Reference) (OtherActor :type Actor%20Object%20Reference) (OtherComp :type Primitive%20Component%20Object%20Reference) (OtherBodyIndex :type Integer) (bFromSweep :type Boolean) (SweepResult :type Hit%20Result%20Structure%20%28by%20ref%29))
  (if (== OtherActor (Variables|Default|GetTPCharacterRef))
    (CallFunction|Cancel)))

(event Custom|OnCancel)

(event EventTick
  (params (DeltaSeconds :type Float%20%28single-precision%29))
  (switch Utilities|FlowControl|Switch|SwitchonE_GrapplingHook (Variables|Default|GetOperatingMode)
    (:NewEnumerator1
      (CallFunction|PullPlayer))
    (:NewEnumerator2
      (CallFunction|PullObject DeltaSeconds)))
  (Variables|Default|GetTPAnimBP
    (:then
      _)
    (:else
      (bind _asepic_character_anim_bp (Utilities|Casting|CastToEpicCharacter_AnimBP (Components|SkeletalMesh|GetAnimInstance (Variables|/Script/Engine.Character|GetMesh (Variables|Default|GetTPCharacterRef)))))
      (Variables|Default|SetTPAnimBP _asepic_character_anim_bp)))
  (Variables|/Game/LearningKit_Games/Assets/Characters/Character/Animations/epicCharacter_AnimBP.EpicCharacter_AnimBP_C|SetBoneLookAtLocation (Variables|Default|GetTPAnimBP) (Transformation|GetWorldLocation (Variables|Default|GetHook))))

(event EventBeginPlay
  (Components|Movement|SetUpdatedComponent (Variables|Default|GetReelRotator) (Variables|Default|GetReel)))

(fn ConstructionScript
  (|CallParentFunction))

(fn Activate
  (|CallParentFunction)
  (Variables|Default|GetTPCharacterRef
    (:then
      _)
    (:else
      (bind _asbp_hour_of_code_character (Utilities|Casting|CastToBP_HourOfCode_Character (Game|GetPlayerCharacter 0)))
      (Variables|Default|SetTPCharacterRef _asbp_hour_of_code_character)))
  (bind (_returnvalue _hitresult) (CallFunction|CheckObjectinRange))
  (if _returnvalue
    (bind _output_get (LocalVariables|SetHitLocation (.Location (Collision|BreakHitResult _hitresult))))
    (Variables|Default|SetGrappledObject (.HitActor (Collision|BreakHitResult _hitresult)))
    (CallFunction|FireHook _output_get)
    (Variables|/Script/Engine.RotatingMovementComponent|SetRotationRate (Variables|Default|GetReelRotator) "0,720.000000, 0")
    (if (Actor|ActorHasTag (Variables|Default|GetGrappledObject) "CanBeGrappled")
      (Variables|Default|SetOperatingMode "NewEnumerator2")
      (else
        (Variables|Default|SetOperatingMode "NewEnumerator1")
        (Character|Jump (Variables|Default|GetTPCharacterRef))))
    (else
      (CallFunction|OnCancel))))

(fn CheckObjectinRange
  (bind _tpcharacterref (Variables|Default|GetTPCharacterRef))
  (bind _followcamera (Variables|/Game/Hour_of_Code/Blueprints/Game/BP_HourOfCode_Character.BP_HourOfCode_Character_C|GetFollowCamera _tpcharacterref))
  (bind _returnvalue (Transformation|GetWorldLocation _followcamera))
  (bind _returnvalue_2 (Math|Vector|GetForwardVector _followcamera))
  (bind (_outhit _returnvalue_3) (Collision|LineTraceByChannel (+ _returnvalue (* _returnvalue_2 3e+02)) (+ _returnvalue (* _returnvalue_2 3.5e+03)) "TraceTypeQuery1" false 0 "None"))
  (return _returnvalue_3 _outhit))

(fn FireHook
  (params (HitLocation :type Vector))
  (Transformation|SetWorldLocation (Variables|Default|GetHook) HitLocation false false)
  (Transformation|AttachComponentToComponent (Variables|Default|GetHook) (Variables|/Script/Engine.Actor|GetRootComponent (Variables|Default|GetGrappledObject)) "None" "KeepWorld" "KeepWorld" "KeepWorld" true)
  (Rendering|SetVisibility (Variables|Default|GetCable) true false))

(fn PullPlayer
  (Variables|/Script/Engine.MovementComponent|SetVelocity (Variables|/Script/Engine.Character|GetCharacterMovement (Variables|Default|GetTPCharacterRef)) (* (Math|Vector|GetUnitDirection(Vector) (Transformation|GetWorldLocation (Variables|/Game/Hour_of_Code/Blueprints/Game/BP_HourOfCode_Character.BP_HourOfCode_Character_C|GetEquipmentLocation (Variables|Default|GetTPCharacterRef))) (Transformation|GetWorldLocation (Variables|Default|GetHook))) (Variables|Default|GetGrappleSpeed))))

(fn PullObject
  (params (DeltaT :type Float%20%28single-precision%29))
  (Transformation|AddActorWorldOffset (Variables|Default|GetGrappledObject) (* (* (Math|Vector|GetUnitDirection(Vector) (Transformation|GetWorldLocation (Variables|Default|GetHook)) (Transformation|GetWorldLocation (Variables|Default|GetHousing))) (Variables|Default|GetGrappleSpeed)) DeltaT)))

(fn Cancel
  (|CallParentFunction)
  (Variables|Default|SetOperatingMode "NewEnumerator0")
  (Transformation|AttachComponentToComponent (Variables|Default|GetHook) (Variables|Default|GetHousing) "None" "SnapToTarget" "SnapToTarget" "SnapToTarget" true)
  (Transformation|SetRelativeLocation (Variables|Default|GetHook) "63.000000, 0,10.000000" false false)
  (Rendering|SetVisibility (Variables|Default|GetCable) false false)
  (Variables|/Script/Engine.RotatingMovementComponent|SetRotationRate (Variables|Default|GetReelRotator) "0, 0, 0")
  (Transformation|SetRelativeRotation (Variables|Default|GetReel) "0, 0, 0" false false)
  (CallFunction|OnCancel))