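; First-person grappling hook equipment that either pulls the player to a hit point or reels tagged objects toward the player.
; Activation line-traces from the camera, attaches the hook to the hit actor, shows the cable, spins the reel, and picks a mode by the CanBeGrappled tag.
; Tick sets player velocity or offsets the object, and feeds the hook location to the anim Blueprint.
; Overlapping the cancel trigger retracts and resets everything.
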(event OnComponentBeginOverlap(HookCancelTrigger)
  (params (OverlappedComponent :type Primitive%20Component%20Object%20Reference) (OtherActor :type Actor%20Object%20Reference) (OtherComp :type Primitive%20Component%20Object%20Reference) (OtherBodyIndex :type Integer) (bFromSweep :type Boolean) (SweepResult :type Hit%20Result%20Structure%20%28by%20ref%29))
  (if (== OtherActor (Variables|Default|GetFPCharacterRef))
    (CallFunction|Cancel)))

(event Custom|OnCancel)

(event EventTick
  (params (DeltaSeconds :type Float%20%28single-precision%29))
  (switch Utilities|FlowControl|Switch|SwitchonE_GrapplingHook (Variables|Default|GetOperatingMode)
    (:NewEnumerator1
      (CallFunction|PullPlayer))
    (:NewEnumerator2
      (CallFunction|PullObject DeltaSeconds)))
  (Variables|Default|GetFPAnimBP
    (:then
      _)
    (:else
      (bind _asfirst_person_anim_bp (Utilities|Casting|CastToFirstPerson_AnimBP (Components|SkeletalMesh|GetAnimInstance (Variables|/Script/Engine.Character|GetMesh (Variables|Default|GetFPCharacterRef)))))
      (Variables|Default|SetFPAnimBP _asfirst_person_anim_bp)))
  (Variables|/Game/FirstPerson/Animations/FirstPerson_AnimBP.FirstPerson_AnimBP_C|SetBoneLookAtLocation (Variables|Default|GetFPAnimBP) (Transformation|GetWorldLocation (Variables|Default|GetHook))))

(event EventBeginPlay
  (Components|Movement|SetUpdatedComponent (Variables|Default|GetReelRotator) (Variables|Default|GetReel)))

(fn ConstructionScript
  (|CallParentFunction))

(fn Activate
  (|CallParentFunction)
  (Variables|Default|GetFPCharacterRef
    (:then
      _)
    (:else
      (bind _asfirst_person_character (Utilities|Casting|CastToFirstPersonCharacter (Game|GetPlayerCharacter 0)))
      (Variables|Default|SetFPCharacterRef _asfirst_person_character)))
  (bind (_returnvalue _hitresult) (CallFunction|CheckObjectinRange))
  (if _returnvalue
    (LocalVariables|SetHitLocation (.Location (Collision|BreakHitResult _hitresult)))
    (Variables|Default|SetGrappledObject (.HitActor (Collision|BreakHitResult _hitresult)))
    (CallFunction|FireHook (LocalVariables|GetHitLocation))
    (Variables|/Script/Engine.RotatingMovementComponent|SetRotationRate (Variables|Default|GetReelRotator) "0,720.000000, 0")
    (if (Actor|ActorHasTag (Variables|Default|GetGrappledObject) "CanBeGrappled")
      (Variables|Default|SetOperatingMode "NewEnumerator2")
      (else
        (Variables|Default|SetOperatingMode "NewEnumerator1")
        (Character|Jump (Variables|Default|GetFPCharacterRef))))
    (else
      (CallFunction|OnCancel))))

(fn CheckObjectinRange
  (bind _fpcharacterref (Variables|Default|GetFPCharacterRef))
  (bind _firstpersoncamera (Variables|/Game/FirstPersonBP/Blueprints/FirstPersonCharacter.FirstPersonCharacter_C|GetFirstPersonCamera _fpcharacterref))
  (bind _returnvalue (Transformation|GetWorldLocation _firstpersoncamera))
  (bind _returnvalue_2 (Math|Vector|GetForwardVector _firstpersoncamera))
  (bind (_outhit _returnvalue_3) (Collision|LineTraceByChannel (+ _returnvalue (* _returnvalue_2 5e+01)) (+ _returnvalue (* _returnvalue_2 3.5e+03)) "TraceTypeQuery1" false 0 "None"))
  (return _returnvalue_3 _outhit))

(fn FireHook
  (params (HitLocation :type Vector))
  (Transformation|SetWorldLocation (Variables|Default|GetHook) HitLocation false false)
  (Transformation|AttachComponentToComponent (Variables|Default|GetHook) (Variables|/Script/Engine.Actor|GetRootComponent (Variables|Default|GetGrappledObject)) "None" "KeepWorld" "KeepWorld" "KeepWorld" true)
  (Rendering|SetVisibility (Variables|Default|GetCable) true false))

(fn PullPlayer
  (Variables|/Script/Engine.MovementComponent|SetVelocity (Variables|/Script/Engine.Character|GetCharacterMovement (Variables|Default|GetFPCharacterRef)) (* (Math|Vector|GetUnitDirection(Vector) (Transformation|GetWorldLocation (Variables|/Game/FirstPersonBP/Blueprints/FirstPersonCharacter.FirstPersonCharacter_C|GetFirstPersonCamera (Variables|Default|GetFPCharacterRef))) (Transformation|GetWorldLocation (Variables|Default|GetHook))) (Variables|Default|GetGrappleSpeed))))

(fn PullObject
  (params (DeltaT :type Float%20%28single-precision%29))
  (Transformation|AddActorWorldOffset (Variables|Default|GetGrappledObject) (* (* (Math|Vector|GetUnitDirection(Vector) (Transformation|GetWorldLocation (Variables|Default|GetHook)) (Transformation|GetWorldLocation (Variables|Default|GetHousing))) (Variables|Default|GetGrappleSpeed)) DeltaT)))

(fn Cancel
  (|CallParentFunction)
  (Variables|Default|SetOperatingMode "NewEnumerator0")
  (Transformation|AttachComponentToComponent (Variables|Default|GetHook) (Variables|Default|GetHousing) "None" "SnapToTarget" "SnapToTarget" "SnapToTarget" true)
  (Transformation|SetRelativeLocation (Variables|Default|GetHook) "63.000000, 0,10.000000" false false)
  (Rendering|SetVisibility (Variables|Default|GetCable) false false)
  (Variables|/Script/Engine.RotatingMovementComponent|SetRotationRate (Variables|Default|GetReelRotator) "0, 0, 0")
  (Transformation|SetRelativeRotation (Variables|Default|GetReel) "0, 0, 0" false false)
  (CallFunction|OnCancel))